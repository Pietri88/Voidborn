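; AI controller for the boss that chases and attacks the player, driven by Tick logic.
; On possess it caches the pawn as a BP_BASE_Enemy.
; While that enemy is aggroed and both sides are alive, it moves straight toward player 0 until within stop distance.
; Within attack range and off cooldown, it sets the enemy's CanAttack flag and turns it toward the player, otherwise clearing the flag.
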(event Custom|SetTargetPlayer
  (params (TargetPawn :type Pawn%20Object%20Reference))
  (Variables|Default|SetTarget%20Pawn TargetPawn))

(event EventBeginPlay
  (|CallParentFunction) ; This node is disabled and will not be called.\nDrag off pins to build functionality.
)

(event EventTick
  (params (DeltaSeconds :type Float%20%28single-precision%29))
  (if (Variables|/Game/Blueprints/Characters/Enemy/BP_BASE_Enemy.BP_BASE_Enemy_C|GetIsInAggro (Variables|Default|GetOwningEnemy))
    (Variables|Default|SetTarget%20Pawn (Game|Player|GetPlayerPawn 0))
    (Utilities|IsValid (Variables|Default|GetTarget%20Pawn)
      (:Is%20Valid
        (bind _asbp_player (Utilities|Casting|CastToBP_Player (Variables|Default|GetTarget%20Pawn)))
        (if (and (not (Variables|/Game/Blueprints/Characters/BP_BASE_CHARACTER.BP_BASE_CHARACTER_C|GetIsDead (Variables|Default|GetOwningEnemy))) (not (Variables|/Game/Blueprints/Characters/BPC_Vitality.BPC_Vitality_C|GetIsDefeated (Variables|/Game/Blueprints/Characters/BP_BASE_CHARACTER.BP_BASE_CHARACTER_C|GetBPC_Vitality _asbp_player))))
          (Utilities|IsValid (Variables|Default|GetOwningEnemy)
            (:Is%20Valid
              (Utilities|IsValid (Variables|Default|GetTarget%20Pawn)
                (:Is%20Valid
                  (Utilities|FlowControl|Sequence
                    (:then_0
                      (if (not (<= (Transformation|GetDistanceTo (Variables|Default|GetOwningEnemy) (Variables|Default|GetTarget%20Pawn)) (Variables|Default|GetDistanceToStopBAttack)))
                        (Default|MoveTowards (Variables|Default|GetOwningEnemy) (Math|Vector|GetForwardVector (Math|Rotator|FindLookatRotation (Transformation|GetActorLocation (Variables|Default|GetOwningEnemy)) (Transformation|GetActorLocation (Variables|Default|GetTarget%20Pawn)))) 1.0)))
                    (:then_1
                      (if (and (<= (Transformation|GetDistanceTo (Variables|Default|GetOwningEnemy) (Variables|Default|GetTarget%20Pawn)) (Variables|Default|GetDistanceToAttack)) (<= (Variables|/Game/Blueprints/Characters/BP_BASE_CHARACTER.BP_BASE_CHARACTER_C|GetAttackCooldown (Variables|Default|GetOwningEnemy)) 0.0))
                        (Variables|/Game/Blueprints/Characters/Enemy/BP_BASE_Enemy.BP_BASE_Enemy_C|SetCanAttack (Variables|Default|GetOwningEnemy) true)
                        ;[1 1 1] Look at enemy when attacking
                        (Default|Lookat (Variables|Default|GetOwningEnemy) (Math|Vector|GetForwardVector (Math|Rotator|FindLookatRotation (Transformation|GetActorLocation (Variables|Default|GetOwningEnemy)) (Transformation|GetActorLocation (Variables|Default|GetTarget%20Pawn)))))
                        (else
                          (Variables|/Game/Blueprints/Characters/Enemy/BP_BASE_Enemy.BP_BASE_Enemy_C|SetCanAttack (Variables|Default|GetOwningEnemy) false))))))))))))))

(event EventPossess
  (params (PossessedPawn :type Pawn%20Object%20Reference))
  (bind _asbp_base_enemy (Utilities|Casting|CastToBP_BASE_Enemy PossessedPawn))
  (Variables|Default|SetOwningEnemy _asbp_base_enemy))

(fn ConstructionScript
  (|CallParentFunction))