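; Action game mode that handles player respawning at checkpoints.
; BeginPlay caches a PlayerStart as the fallback spawn point.
; RespawnPlayer spawns a new default pawn at the active checkpoint's Scene component, or at that PlayerStart when no checkpoint is valid.
; Player controller 0 possesses the new BP_Player, whose health is refilled and defeated and dead flags are cleared.
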(event EventBeginPlay
  (bind _returnvalue (Actor|GetActorOfClass "/Script/Engine.PlayerStart"))
  (Variables|Default|SetPlayerStart _returnvalue))

(event EventTick
  (params (DeltaSeconds :type Float%20%28single-precision%29)))

(fn ConstructionScript)

(fn RespawnPlayer
  (bind _playerstart (Variables|Default|GetPlayerStart))
  (bind _activecheckpoint (Variables|Default|GetActiveCheckpoint))
  (bind _returnvalue (Transformation|GetActorTransform _playerstart))
  (bind _scene (Variables|/Game/Blueprints/Props/BP_Checkpoint.BP_Checkpoint_C|GetScene _activecheckpoint))
  (bind _returnvalue_2 (Transformation|GetWorldTransform _scene))
  (Utilities|IsValid _activecheckpoint
    (:Is%20Valid
      (bind _returnvalue_3 (Game|SpawnActorfromClass (Variables|Default|GetDefaultPawnClass) (Math|Transform|MakeTransform (.location _returnvalue_2) (.rotation _returnvalue_2) "1.000000,1.000000,1.000000") "AlwaysSpawn" "MultiplyWithRoot" 0 0))
      (bind _asbp_player (Utilities|Casting|CastToBP_Player _returnvalue_3))
      (Pawn|Possess (Game|GetPlayerController 0) _returnvalue_3)
      (Variables|/Game/Blueprints/Characters/BPC_Vitality.BPC_Vitality_C|SetIsDefeated (Variables|/Game/Blueprints/Characters/BP_BASE_CHARACTER.BP_BASE_CHARACTER_C|GetBPC_Vitality _asbp_player) false)
      (Variables|/Game/Blueprints/Characters/BPC_Vitality.BPC_Vitality_C|SetCurrentHealth (Variables|/Game/Blueprints/Characters/BP_BASE_CHARACTER.BP_BASE_CHARACTER_C|GetBPC_Vitality _asbp_player) (Variables|/Game/Blueprints/Characters/BPC_Vitality.BPC_Vitality_C|GetMaxHealth (Variables|/Game/Blueprints/Characters/BP_BASE_CHARACTER.BP_BASE_CHARACTER_C|GetBPC_Vitality _asbp_player)))
      (Variables|/Game/Blueprints/Characters/BP_BASE_CHARACTER.BP_BASE_CHARACTER_C|SetIsDead _asbp_player false))
    (:Is%20Not%20Valid
      (bind _returnvalue_4 (Game|SpawnActorfromClass (Variables|Default|GetDefaultPawnClass) (Math|Transform|MakeTransform (.location _returnvalue) (.rotation _returnvalue) "1.000000,1.000000,1.000000") "AlwaysSpawn" "MultiplyWithRoot" 0 0))
      (bind _asbp_player_2 (Utilities|Casting|CastToBP_Player _returnvalue_4))
      (Pawn|Possess (Game|GetPlayerController 0) _returnvalue_4)
      (Variables|/Game/Blueprints/Characters/BPC_Vitality.BPC_Vitality_C|SetIsDefeated (Variables|/Game/Blueprints/Characters/BP_BASE_CHARACTER.BP_BASE_CHARACTER_C|GetBPC_Vitality _asbp_player_2) false)
      (Variables|/Game/Blueprints/Characters/BPC_Vitality.BPC_Vitality_C|SetCurrentHealth (Variables|/Game/Blueprints/Characters/BP_BASE_CHARACTER.BP_BASE_CHARACTER_C|GetBPC_Vitality _asbp_player_2) (Variables|/Game/Blueprints/Characters/BPC_Vitality.BPC_Vitality_C|GetMaxHealth (Variables|/Game/Blueprints/Characters/BP_BASE_CHARACTER.BP_BASE_CHARACTER_C|GetBPC_Vitality _asbp_player_2)))
      (Variables|/Game/Blueprints/Characters/BP_BASE_CHARACTER.BP_BASE_CHARACTER_C|SetIsDead _asbp_player_2 false))))