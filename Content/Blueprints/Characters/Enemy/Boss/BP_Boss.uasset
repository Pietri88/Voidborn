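; Boss enemy that binds its health widget on BeginPlay and damages opposing-faction players entering its attack radius while HitPlayer is set.
; AnyDamage drives one-shot health-threshold phases: teleport and cast, shield while spawning two enemies, then transform with a full heal.
; In phase 2, half health triggers a timed, floating, collision-free summon.
; Phases use animation state jumps and delays; shielding or a pending teleport blocks parent damage handling.
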(event OnComponentBeginOverlap(AttackRadius)
  (params (OverlappedComponent :type Primitive%20Component%20Object%20Reference) (OtherActor :type Actor%20Object%20Reference) (OtherComp :type Primitive%20Component%20Object%20Reference) (OtherBodyIndex :type Integer) (bFromSweep :type Boolean) (SweepResult :type Hit%20Result%20Structure%20%28by%20ref%29))
  (bind _asbp_player (Utilities|Casting|CastToBP_Player OtherActor))
  (if (Utilities|Enum|NotEqual(Enum) (Variables|/Game/Blueprints/Characters/BP_BASE_CHARACTER.BP_BASE_CHARACTER_C|GetFaction _asbp_player) (Variables|Default|GetFaction))
    (if (Variables|Default|GetHitPlayer)
      (Game|Damage|ApplyDamage _asbp_player 1.0 0 self))))

(event EventBeginPlay
  (|CallParentFunction)
  (bind _aswbp_boss_health (Utilities|Casting|CastToWBP_BossHealth (UserInterface|GetUserWidgetObject (Variables|Default|GetWidget))))
  (Variables|/Game/Widgets/WBP_BossHealth.WBP_BossHealth_C|SetBossActor _aswbp_boss_health self)
  (bind _asbp_player (Utilities|Casting|CastToBP_Player (Game|Player|GetPlayerPawn 0)))
  (Variables|Default|SetPlayer _asbp_player))

(event Collision|EventActorBeginOverlap
  (params (OtherActor :type Actor%20Object%20Reference))
  (|CallParentFunction OtherActor) ; This node is disabled and will not be called.\nDrag off pins to build functionality.
)

(event EventTick
  (params (DeltaSeconds :type Float%20%28single-precision%29))
  (|CallParentFunction DeltaSeconds))

(event Game|Damage|EventAnyDamage
  (params (Damage :type Float%20%28single-precision%29) (DamageType :type Damage%20Type%20Object%20Reference) (InstigatedBy :type Controller%20Object%20Reference) (DamageCauser :type Actor%20Object%20Reference))
  (bind _returnvalue (Transformation|GetActorLocation))
  (bind _returnvalue_2 (Transformation|GetActorLocation))
  (bind _bpc_vitality (Variables|Default|GetBPC_Vitality))
  (bind _bpc_vitality_2 (Variables|Default|GetBPC_Vitality))
  (bind _bpc_vitality_3 (Variables|Default|GetBPC_Vitality))
  (bind _bpc_vitality_4 (Variables|Default|GetBPC_Vitality))
  (bind _bpc_vitality_5 (Variables|Default|GetBPC_Vitality))
  (if (not (Variables|Default|GetIsShielding))
    (if (not (Variables|Default|GetHasToTeleport))
      (|CallParentFunction Damage 0 0 0)
      (Utilities|FlowControl|Sequence
        (:then_0
          (if (<= (Variables|/Game/Blueprints/Characters/BPC_Vitality.BPC_Vitality_C|GetCurrentHealth _bpc_vitality_3) (* (Variables|/Game/Blueprints/Characters/BPC_Vitality.BPC_Vitality_C|GetMaxHealth _bpc_vitality_3) 0.8))
            (Utilities|FlowControl|DoOnce false
              (:Completed
                (Variables|Default|SetHasToTeleport true)
                (Class|PaperZDAnimInstance|JumptoNode (Variables|/Script/PaperZD.PaperZDAnimationComponent|GetAnimInstance (Variables|Default|GetAnimationComponent)) "JumpTeleport" "")
                (Variables|Default|SetCastingPhase true)
                (Utilities|FlowControl|Delay 6.0)
                (Variables|Default|SetCastingPhase false)
                (Variables|Default|SetHasToTeleportBack true)
                (Class|PaperZDAnimInstance|JumptoNode (Variables|/Script/PaperZD.PaperZDAnimationComponent|GetAnimInstance (Variables|Default|GetAnimationComponent)) "JumpTeleport" "")))))
        (:then_1
          (if (<= (Variables|/Game/Blueprints/Characters/BPC_Vitality.BPC_Vitality_C|GetCurrentHealth _bpc_vitality_2) (* (Variables|/Game/Blueprints/Characters/BPC_Vitality.BPC_Vitality_C|GetMaxHealth _bpc_vitality_2) 0.5))
            (Utilities|FlowControl|DoOnce false
              (:Completed
                (Variables|Default|SetIsShielding true)
                (Class|PaperZDAnimInstance|JumptoNode (Variables|/Script/PaperZD.PaperZDAnimationComponent|GetAnimInstance (Variables|Default|GetAnimationComponent)) "JumpShield" "")
                (Game|SpawnActorfromClass "/Game/Blueprints/Characters/Enemy/EnemyPrototype/BP_EnemyPrototype.BP_EnemyPrototype_C" (Math|Transform|MakeTransform "4315.578451,-50.000000,790.481860" "0, 0, 0" "1.000000,1.000000,1.000000") "AlwaysSpawn" "MultiplyWithRoot" 0 0)
                (Game|SpawnActorfromClass "/Game/Blueprints/Characters/Enemy/EnemyPrototype/BP_EnemyPrototype.BP_EnemyPrototype_C" (Math|Transform|MakeTransform "4460.252568,-50.000000,1410.759563" "0, 0, 0" "1.000000,1.000000,1.000000") "AlwaysSpawn" "MultiplyWithRoot" 0 0)
                (Utilities|FlowControl|Delay 1e+01)
                (Variables|Default|SetIsShielding false)))))
        (:then_2
          (if (<= (Variables|/Game/Blueprints/Characters/BPC_Vitality.BPC_Vitality_C|GetCurrentHealth _bpc_vitality) (/ (Variables|/Game/Blueprints/Characters/BPC_Vitality.BPC_Vitality_C|GetMaxHealth _bpc_vitality) 3.0))
            (Utilities|FlowControl|DoOnce false
              (:Completed
                (Variables|Default|SetIsTransforming true)
                (Class|PaperZDAnimInstance|JumptoNode (Variables|/Script/PaperZD.PaperZDAnimationComponent|GetAnimInstance (Variables|Default|GetAnimationComponent)) "JumpTransform" "")
                (Variables|/Game/Blueprints/Characters/BPC_Vitality.BPC_Vitality_C|SetCurrentHealth _bpc_vitality_5 (Variables|/Game/Blueprints/Characters/BPC_Vitality.BPC_Vitality_C|GetMaxHealth _bpc_vitality_5))))))
        (:then_3
          (if (and (<= (Variables|/Game/Blueprints/Characters/BPC_Vitality.BPC_Vitality_C|GetCurrentHealth _bpc_vitality_4) (* (Variables|/Game/Blueprints/Characters/BPC_Vitality.BPC_Vitality_C|GetMaxHealth _bpc_vitality_4) 0.5)) (Variables|Default|GetIsInPhase2))
            (Utilities|FlowControl|DoOnce false
              (:Completed
                (Variables|Default|SetIsInSummoningPhase true)
                (Transformation|Teleport (Math|Vector|MakeVector (.x _returnvalue) (.y _returnvalue) (+ (.z _returnvalue) 1e+02)) "0, 0, 0")
                (Variables|/Script/Engine.CharacterMovementComponent|SetGravityScale (Variables|Character|GetCharacterMovement) 0.0)
                (Collision|SetCollisionEnabled (Variables|Default|GetCapsuleComponent) "NoCollision")
                (Class|PaperZDAnimInstance|JumptoNode (Variables|/Script/PaperZD.PaperZDAnimationComponent|GetAnimInstance (Variables|Default|GetAnimationComponent)) "JumpSummon" "")
                (Utilities|FlowControl|Delay 3.0)
                (Variables|Default|SetIsInSummoningPhase false)
                (Variables|/Script/Engine.CharacterMovementComponent|SetGravityScale (Variables|Character|GetCharacterMovement) 3.0)
                (Collision|SetCollisionEnabled (Variables|Default|GetCapsuleComponent) "QueryAndPhysics")
                (Transformation|Teleport (Math|Vector|MakeVector (.x _returnvalue_2) (.y _returnvalue_2) (- (.z _returnvalue_2) 8e+01)) "0, 0, 0")))))))
    (else
      (Class|PaperZDAnimInstance|JumptoNode (Variables|/Script/PaperZD.PaperZDAnimationComponent|GetAnimInstance (Variables|Default|GetAnimationComponent)) "JumpHurt" "None"))))

(fn ConstructionScript
  (|CallParentFunction))