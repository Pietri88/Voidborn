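; Necromancer enemy Blueprint, a child class that adds a ranged projectile attack.
; BeginPlay runs the parent logic, then sets AttackCooldown from DefaultAttackCooldown.
; SpawnProjectile spawns BP_Projectile_Enemy at the SpawnFireball component's world location and rotation, ignoring collisions; nothing in this Blueprint calls it.
; Tick and the construction script only call their parents.
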(event EventBeginPlay
  (|CallParentFunction)
  (Variables|Default|SetAttackCooldown (Variables|Default|GetDefaultAttackCooldown)))

(event Collision|EventActorBeginOverlap
  (params (OtherActor :type Actor%20Object%20Reference))
  (|CallParentFunction OtherActor) ; This node is disabled and will not be called.\nDrag off pins to build functionality.
)

(event EventTick
  (params (DeltaSeconds :type Float%20%28single-precision%29))
  (|CallParentFunction DeltaSeconds))

(fn ConstructionScript
  (|CallParentFunction))

(fn SpawnProjectile
  (bind _spawnfireball (Variables|Default|GetSpawnFireball))
  (Game|SpawnActorfromClass "/Game/Blueprints/Projectiles/BP_Projectile_Enemy.BP_Projectile_Enemy_C" (Math|Transform|MakeTransform (Transformation|GetWorldLocation _spawnfireball) (Transformation|GetWorldRotation _spawnfireball) "1.000000,1.000000,1.000000") "AlwaysSpawn" "MultiplyWithRoot" 0 0))