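; Base enemy character for side-on movement along X, flipping to face its direction and turning at walls and ledges.
; Each tick, line traces for walls, ground and landing spots feed a check that triggers jumps.
; Overlap volumes track player range and aggro, passing the player to melee or ranged AI controllers and gating MoveTowards movement.
; Damage sets a timed stun, with a stun animation unless defeated.
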(event OnComponentBeginOverlap(PlayerDettector)
  (params (OverlappedComponent :type Primitive%20Component%20Object%20Reference) (OtherActor :type Actor%20Object%20Reference) (OtherComp :type Primitive%20Component%20Object%20Reference) (OtherBodyIndex :type Integer) (bFromSweep :type Boolean) (SweepResult :type Hit%20Result%20Structure%20%28by%20ref%29))
  (Utilities|Casting|CastToBP_Player OtherActor)
  (Variables|Default|SetIsInPlayerRange true))

(event OnComponentBeginOverlap(AgrroRadius)
  (params (OverlappedComponent :type Primitive%20Component%20Object%20Reference) (OtherActor :type Actor%20Object%20Reference) (OtherComp :type Primitive%20Component%20Object%20Reference) (OtherBodyIndex :type Integer) (bFromSweep :type Boolean) (SweepResult :type Hit%20Result%20Structure%20%28by%20ref%29))
  (bind _self self)
  (bind _returnvalue (AI|GetAIController _self))
  (bind _asbp_player (Utilities|Casting|CastToBP_Player OtherActor))
  (Variables|Default|SetowningEnemy _asbp_player)
  (Variables|Default|SetIsInAggro true)
  (Utilities|FlowControl|DoOnce false :!label _label
    (:Completed
      (Utilities|Casting|CastToAIC_Base _returnvalue)
      (Utilities|FlowControl|Sequence
        (:then_0
          (bind _asaic_base_melee (Utilities|Casting|CastToAIC_BaseMelee _returnvalue))
          (Default|SetTargetPlayer _asaic_base_melee _asbp_player))
        (:then_1
          (bind _asaic_base_ranged (Utilities|Casting|CastToAIC_BaseRanged _returnvalue))
          (Default|SetTargetPlayer _asaic_base_ranged _asbp_player)))
      (if (not (Variables|/Game/Blueprints/Characters/BP_BASE_CHARACTER.BP_BASE_CHARACTER_C|GetIsDead _asbp_player))
        (goto _label Reset)))))

(event OnComponentEndOverlap(PlayerDettector)
  (params (OverlappedComponent :type Primitive%20Component%20Object%20Reference) (OtherActor :type Actor%20Object%20Reference) (OtherComp :type Primitive%20Component%20Object%20Reference) (OtherBodyIndex :type Integer))
  (Utilities|Casting|CastToBP_Player OtherActor)
  (Variables|Default|SetIsInPlayerRange false))

(event OnComponentBeginOverlap(WallDetector)
  (params (OverlappedComponent :type Primitive%20Component%20Object%20Reference) (OtherActor :type Actor%20Object%20Reference) (OtherComp :type Primitive%20Component%20Object%20Reference) (OtherBodyIndex :type Integer) (bFromSweep :type Boolean) (SweepResult :type Hit%20Result%20Structure%20%28by%20ref%29))
  (Utilities|FlowControl|DoOnce false
    (:Completed
      (CallFunction|TurnCharacter))))

(event OnComponentEndOverlap(LedgeDetector)
  (params (OverlappedComponent :type Primitive%20Component%20Object%20Reference) (OtherActor :type Actor%20Object%20Reference) (OtherComp :type Primitive%20Component%20Object%20Reference) (OtherBodyIndex :type Integer))
  (CallFunction|TurnCharacter))

(event OnComponentEndOverlap(AgrroRadius)
  (params (OverlappedComponent :type Primitive%20Component%20Object%20Reference) (OtherActor :type Actor%20Object%20Reference) (OtherComp :type Primitive%20Component%20Object%20Reference) (OtherBodyIndex :type Integer))
  (Utilities|Casting|CastToBP_Player OtherActor)
  (Variables|Default|SetIsInAggro false))

(event Custom|MoveTowards
  (params (WorldDirection :type Vector) (ScaleValue :type Float%20%28single-precision%29))
  (bind _charactermovement (Variables|Character|GetCharacterMovement))
  (if (and (Variables|Default|GetIsInAggro) (not (Variables|Default|GetIsStayingOnEdge)))
    (Pawn|Input|AddMovementInput WorldDirection ScaleValue false))
  (Transformation|SetActorRotation (select (< (.X (Math|Vector|BreakVector WorldDirection)) 0.0) "0.000000,180.000000,0.000000" "0, 0, 0"))
  (Variables|/Script/Engine.CharacterMovementComponent|SetMaxWalkSpeed _charactermovement 6e+02)
  (Variables|/Script/Engine.CharacterMovementComponent|SetMaxFlySpeed _charactermovement 6e+02))

(event Custom|LookAt
  (params (Direction :type Vector))
  (Transformation|SetActorRotation (select (< (.X (Math|Vector|BreakVector Direction)) 0.0) "0.000000,180.000000,0.000000" "0, 0, 0")))

(event Custom|WalkForward
  (params (ScaleValue :type Float%20%28single-precision%29))
  (Pawn|Input|AddMovementInput (Transformation|GetActorForwardVector) ScaleValue false))

(event EventBeginPlay
  (|CallParentFunction)
  (Variables|Default|SetFaction "NewEnumerator1"))

(event Collision|EventActorBeginOverlap
  (params (OtherActor :type Actor%20Object%20Reference))
  (|CallParentFunction OtherActor) ; This node is disabled and will not be called.\nDrag off pins to build functionality.
)

(event EventTick
  (params (DeltaSeconds :type Float%20%28single-precision%29))
  (bind _returnvalue (Transformation|GetActorLocation))
  (bind _returnvalue_2 (Transformation|GetActorForwardVector))
  (bind _returnvalue_3 (Transformation|GetActorLocation))
  (bind _walltracelengthoffsetz (Variables|Default|GetWallTraceLengthOffsetZ))
  (bind _returnvalue_4 (+ (.z _returnvalue) _walltracelengthoffsetz))
  (|CallParentFunction DeltaSeconds)
  (bind _returnvalue_5 (Collision|LineTraceForObjects (Math|Vector|MakeVector (.x _returnvalue) (.y _returnvalue) _returnvalue_4) (+ (Math|Vector|MakeVector (.x _returnvalue) (.y _returnvalue) _returnvalue_4) (* (Math|Vector|MakeVector (.x _returnvalue_2) (.y _returnvalue_2) (.z _returnvalue_2)) (Variables|Default|GetWallTraceLength))) (Utilities|Array|MakeArray "ObjectTypeQuery1") false 0 "None"))
  ;[1 1 1] Track wall ahead of player
  (bind _returnvalue_6 (Collision|LineTraceForObjects _returnvalue_3 (+ _returnvalue_3 (* (Transformation|GetActorForwardVector) (Variables|Default|GetWallTraceLength))) (Utilities|Array|MakeArray "ObjectTypeQuery1") false 0 "None"))
  (|CheckForGround
    (:execute
      (|CheckForPlaceToLand)
      (if (|BeforeJumpChecks (not _returnvalue_5) _returnvalue_6)
        (Character|Jump)
        (Variables|Default|SetJumpCooldown 1.0)))))

(event Game|Damage|EventAnyDamage
  (params (Damage :type Float%20%28single-precision%29) (DamageType :type Damage%20Type%20Object%20Reference) (InstigatedBy :type Controller%20Object%20Reference) (DamageCauser :type Actor%20Object%20Reference))
  (|CallParentFunction Damage 0 0 0)
  ;[1 1 1] Stunowanie wrogów
  (Variables|Default|SetIsStunned true)
  (if (not (Variables|/Game/Blueprints/Characters/BPC_Vitality.BPC_Vitality_C|GetIsDefeated (Variables|Default|GetBPC_Vitality)))
    (Class|PaperZDAnimInstance|JumptoNode (Variables|/Script/PaperZD.PaperZDAnimationComponent|GetAnimInstance (Variables|Default|GetAnimationComponent)) "JumpStun" "None")
    (Utilities|FlowControl|Delay (Variables|Default|GetStunDuration))
    (Variables|Default|SetIsStunned false)))

(fn ConstructionScript
  (|CallParentFunction))

(fn TurnCharacter
  (Transformation|SetActorRotation (Math|Rotator|CombineRotators (Transformation|GetActorRotation) "0.000000,180.000000,0.000000")))