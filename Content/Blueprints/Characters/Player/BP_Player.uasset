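; Player character for a side-scrolling action game, with run, wall slide and jump, dash, attack, block and counter.
; Enhanced Input sets state flags and triggers animation node jumps, while Tick updates HUD bars, cooldowns, wall-slide traces and slow stamina regen.
; Dash and block spend BPCVitality stamina; countered hits spawn a deflected projectile, other unblocked damage can lead to a fade and GM_Action respawn.
; Also creates and removes the boss health bar.
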(event OnComponentBeginOverlap(AttackRadius)
  (params (OverlappedComponent :type Primitive%20Component%20Object%20Reference) (OtherActor :type Actor%20Object%20Reference) (OtherComp :type Primitive%20Component%20Object%20Reference) (OtherBodyIndex :type Integer) (bFromSweep :type Boolean) (SweepResult :type Hit%20Result%20Structure%20%28by%20ref%29))
  (bind _asbp_base_enemy (Utilities|Casting|CastToBP_BASE_Enemy OtherActor))
  (if (Utilities|Enum|NotEqual(Enum) (Variables|/Game/Blueprints/Characters/BP_BASE_CHARACTER.BP_BASE_CHARACTER_C|GetFaction _asbp_base_enemy) (Variables|Default|GetFaction))
    (if (Variables|Default|GetHitEnemy)
      (Game|Damage|ApplyDamage _asbp_base_enemy 1.0 0 self))))

(event OnComponentBeginOverlap(CapsuleComponent)
  (params (OverlappedComponent :type Primitive%20Component%20Object%20Reference) (OtherActor :type Actor%20Object%20Reference) (OtherComp :type Primitive%20Component%20Object%20Reference) (OtherBodyIndex :type Integer) (bFromSweep :type Boolean) (SweepResult :type Hit%20Result%20Structure%20%28by%20ref%29))
  (Utilities|Casting|CastToSpell1 OtherActor)
  (Variables|Default|SetGotHitBySpell true))

(event OnComponentEndOverlap(CapsuleComponent)
  (params (OverlappedComponent :type Primitive%20Component%20Object%20Reference) (OtherActor :type Actor%20Object%20Reference) (OtherComp :type Primitive%20Component%20Object%20Reference) (OtherBodyIndex :type Integer))
  (Utilities|Casting|CastToSpell1 OtherActor)
  (Variables|Default|SetGotHitBySpell false))

(event Custom|PredeterminedJump
  (params (JumpDirection :type Float%20%28double-precision%29))
  (Character|LaunchCharacter (Math|Vector|MakeVector (* (.x (Transformation|GetActorForwardVector)) (Variables|Default|GetWallJumpPowerHor) JumpDirection) 0.0 (Variables|Default|GetJumpPowerVert)) false false))

(event Custom|SetDashOnCD
  (Variables|Default|SetDashCooldown (- (Variables|Default|GetDashCooldown) (Utilities|Time|GetWorldDeltaSeconds)))
  (if (<= (Math|Float|Absolute(Float) (.x (Variables|/Script/Engine.MovementComponent|GetVelocity (Variables|Character|GetCharacterMovement)))) (+ (Variables|Default|GetBaseRunSpeed) 7e+02))
    (Variables|/Script/Engine.CharacterMovementComponent|SetGravityScale (Variables|Character|GetCharacterMovement) (Variables|Default|GetBaseGravity))
    (Variables|Default|SetIsDashing false)
    (Utilities|FlowControl|Sequence
      (:then_0
        (if (<= (Variables|Default|GetDashCooldown) 0.0)
          (Variables|Default|SetIsDashOnCd false))))))

(event Custom|SpawnBossHealthBar
  (params (BossRef :type BP%20Boss%20Object%20Reference))
  (bind _returnvalue (UserInterface|CreateWidget "/Game/Widgets/WBP_BossHealth.WBP_BossHealth_C" 0 BossRef))
  (bind _output_get (Variables|Default|SetBossBarRef _returnvalue))
  (UserInterface|Viewport|AddtoViewport _output_get 0))

(event Custom|RemoveBossHealthBar
  (Utilities|IsValid (Variables|Default|GetBossBarRef)
    (:Is%20Valid
      (Widget|RemovefromParent (Variables|Default|GetBossBarRef)))))

(event Input|EnhancedActionEvents|EnhancedInputActionIA_Move
  (params (ActionValue :type Vector%202D%20Structure) (ElapsedSeconds :type Float%20%28double-precision%29) (TriggeredSeconds :type Float%20%28double-precision%29) (InputAction :type Input%20Action%20Object%20Reference :default "/Game/Input/Actions/IA_Move.IA_Move"))
  (if (not (Variables|Default|GetIsBlocking))
    (Pawn|Input|AddMovementInput "1.000000,0.000000,0.000000" (.x ActionValue) false)
    (Pawn|SetControlRotation (Pawn|GetController) (select (>= (.x ActionValue) 0.0) (Math|Rotator|MakeRotator 0.0 0.0 0.0) (Math|Rotator|MakeRotator 0.0 0.0 1.8e+02)))))

(event Input|EnhancedActionEvents|EnhancedInputActionIA_Jump
  (params (ActionValue :type Boolean) (ElapsedSeconds :type Float%20%28double-precision%29) (TriggeredSeconds :type Float%20%28double-precision%29) (InputAction :type Input%20Action%20Object%20Reference :default "/Game/Input/Actions/IA_Jump.IA_Jump"))
  (:Started
    (if (Variables|Default|GetIsWallSliding)
      (CallFunction|PredeterminedJump -1.0)
      (elif (not (Variables|Default|GetIsBlocking))
        (Character|Jump)))))

(event Input|EnhancedActionEvents|EnhancedInputActionIA_Attack
  (params (ActionValue :type Boolean) (ElapsedSeconds :type Float%20%28double-precision%29) (TriggeredSeconds :type Float%20%28double-precision%29) (InputAction :type Input%20Action%20Object%20Reference :default "/Game/Input/Actions/IA_Attack.IA_Attack"))
  (bind _charactermovement (Variables|Character|GetCharacterMovement))
  (:Started
    (if (Math|Boolean|ANDBoolean (not (Variables|Default|GetIsWallSliding)) (not (Variables|Default|GetIsAttacking)) (not (Variables|Default|GetIsCountering)))
      (Variables|Default|SetbUseControllerRotationYaw false)
      (Variables|Default|SetIsAttacking true)
      (Class|PaperZDAnimInstance|JumptoNode (Variables|/Script/PaperZD.PaperZDAnimationComponent|GetAnimInstance (Variables|Default|GetAnimationComponent)) "JumpAttack" "None")
      ;[1 1 1] Slowing speed during attacking
      (Variables|/Script/Engine.CharacterMovementComponent|SetMaxWalkSpeed _charactermovement (* (Variables|/Script/Engine.CharacterMovementComponent|GetMaxWalkSpeed _charactermovement) (Variables|Default|GetSpeedDuringAttack))))))

(event Input|EnhancedActionEvents|EnhancedInputActionIA_Dash
  (params (ActionValue :type Boolean) (ElapsedSeconds :type Float%20%28double-precision%29) (TriggeredSeconds :type Float%20%28double-precision%29) (InputAction :type Input%20Action%20Object%20Reference :default "/Game/Input/Actions/IA_Dash.IA_Dash"))
  (bind _charactermovement (Variables|Character|GetCharacterMovement))
  (bind _bpc_vitality (Variables|Default|GetBPC_Vitality))
  (if (Math|Boolean|ANDBoolean (not (Variables|Default|GetIsCountering)) (not (Variables|Default|GetIsDashOnCd)) (<= (Variables|Default|GetDashStaminaCost) (Variables|/Game/Blueprints/Characters/BPC_Vitality.BPC_Vitality_C|GetCurrentStamina (Variables|Default|GetBPC_Vitality))))
    (Variables|Default|SetbUseControllerRotationYaw false)
    (Variables|Default|SetIsDashing true)
    (Collision|SetCollisionResponsetoChannel (Variables|Default|GetCapsuleComponent) "ECC_Pawn" "ECR_Ignore")
    (Variables|/Script/Engine.CharacterMovementComponent|SetGravityScale (Variables|Character|GetCharacterMovement) 0.0)
    (Variables|/Script/Engine.MovementComponent|SetVelocity _charactermovement (Math|Vector|MakeVector (.x (Variables|/Script/Engine.MovementComponent|GetVelocity _charactermovement)) 0.0 0.0))
    (Character|LaunchCharacter (Math|Vector|MakeVector (* (.x (Transformation|GetActorForwardVector)) (Variables|Default|GetDashStrength)) 0.0 0.0) false false)
    (Class|PaperZDAnimInstance|JumptoNode (Variables|/Script/PaperZD.PaperZDAnimationComponent|GetAnimInstance (Variables|Default|GetAnimationComponent)) "JUMP/Dash" "None")
    (Variables|/Game/Blueprints/Characters/BPC_Vitality.BPC_Vitality_C|SetCurrentStamina _bpc_vitality (- (Variables|/Game/Blueprints/Characters/BPC_Vitality.BPC_Vitality_C|GetCurrentStamina _bpc_vitality) (Variables|Default|GetDashStaminaCost)))
    (Variables|Default|SetIsDashOnCd true)
    (Variables|Default|SetDashCooldown (Variables|Default|GetBaseDashCooldown))
    (Variables|Default|SetbUseControllerRotationYaw true)))

(event Input|EnhancedActionEvents|EnhancedInputActionIA_Block
  (params (ActionValue :type Boolean) (ElapsedSeconds :type Float%20%28double-precision%29) (TriggeredSeconds :type Float%20%28double-precision%29) (InputAction :type Input%20Action%20Object%20Reference :default "/Game/Input/Actions/IA_Block.IA_Block"))
  (:Started
    (if (and (not (Variables|Default|GetIsWallSliding)) (not (Variables|Default|GetIsAttacking)))
      (Variables|Default|SetIsBlocking true)
      (Class|PaperZDAnimInstance|JumptoNode (Variables|/Script/PaperZD.PaperZDAnimationComponent|GetAnimInstance (Variables|Default|GetAnimationComponent)) "Jump_Block" "None")))
  (:Canceled
    (Variables|Default|SetIsBlocking false :!label _label))
  (:Completed
    (goto _label)))

(event Input|EnhancedActionEvents|EnhancedInputActionIA_CounterBlock
  (params (ActionValue :type Boolean) (ElapsedSeconds :type Float%20%28double-precision%29) (TriggeredSeconds :type Float%20%28double-precision%29) (InputAction :type Input%20Action%20Object%20Reference :default "/Game/Input/Actions/IA_CounterBlock.IA_CounterBlock"))
  (if (Math|Boolean|ANDBoolean (not (Variables|Default|GetIsWallSliding)) (not (Variables|Default|GetIsAttacking)) (<= (Variables|Default|GetCounterCooldown) 0.0))
    (Variables|Default|SetIsCountering true)
    (Class|PaperZDAnimInstance|JumptoNode (Variables|/Script/PaperZD.PaperZDAnimationComponent|GetAnimInstance (Variables|Default|GetAnimationComponent)) "Jump_Counter" "None")
    (Variables|Default|SetCounterCooldown 2.0)))

(event EventBeginPlay
  (bind _bpc_vitality (Variables|Default|GetBPC_Vitality))
  (|CallParentFunction)
  (Variables|/Game/Blueprints/Characters/BPC_Vitality.BPC_Vitality_C|SetCurrentStamina _bpc_vitality (Variables|/Game/Blueprints/Characters/BPC_Vitality.BPC_Vitality_C|GetMaxStamina _bpc_vitality))
  (bind _asgm_action (Utilities|Casting|CastToGM_Action (Game|GetGameMode)))
  (Variables|Default|SetGM%20Action _asgm_action)
  (bind _asplayer_controller (Utilities|Casting|CastToPlayerController (Pawn|GetController)))
  (Input|AddMappingContext (PlayerController|LocalPlayerSubsystems|GetEnhancedInputLocalPlayerSubsystem _asplayer_controller) "/Game/Input/IMC_Action.IMC_Action" 0 "(bIgnoreAllPressedKeysUntilRelease=True,bForceImmediately=False,bNotifyUserSettings=False)")
  (Variables|Default|SetBaseLateralFriction (Variables|/Script/Engine.CharacterMovementComponent|GetFallingLateralFriction (Variables|Character|GetCharacterMovement)))
  (Variables|Default|SetBaseRunSpeed (Class|MovementComponent|GetMaxSpeed (Variables|Character|GetCharacterMovement)))
  (Variables|Default|SetDashCooldown 0.0)
  (Variables|Default|SetFaction "NewEnumerator0")
  (Variables|Default|SetBaseGravity (Variables|/Script/Engine.CharacterMovementComponent|GetGravityScale (Variables|Character|GetCharacterMovement)))
  (Variables|Default|SetCounterCooldown 0.0))

(event Collision|EventActorBeginOverlap
  (params (OtherActor :type Actor%20Object%20Reference)))

(event EventTick
  (params (DeltaSeconds :type Float%20%28single-precision%29))
  (bind _gm_action (Variables|Default|GetGM%20Action))
  (bind _bpc_vitality (Variables|Default|GetBPC_Vitality))
  (bind _hudwidget (Variables|/Game/Blueprints/GM_Action.GM_Action_C|GetHudWidget _gm_action))
  (|CallParentFunction 0.0)
  (Default|UpdateHealth (Variables|/Game/Widgets/WBP_HUD.WBP_HUD_C|GetWBP_HealthComponent _hudwidget) (Variables|/Game/Blueprints/Characters/BPC_Vitality.BPC_Vitality_C|GetCurrentHealth (Variables|Default|GetBPC_Vitality)))
  (Default|UpdateStamina (Variables|/Game/Widgets/WBP_HUD.WBP_HUD_C|GetWBP_StaminaComponent _hudwidget) (Variables|/Game/Blueprints/Characters/BPC_Vitality.BPC_Vitality_C|GetCurrentStamina (Variables|Default|GetBPC_Vitality)))
  (if (Variables|/Game/Blueprints/Characters/BPC_Vitality.BPC_Vitality_C|GetIsDefeated (Variables|Default|GetBPC_Vitality))
    (Input|DisableInput 0)
    (else
      (CallFunction|SetDashonCD)
      (CallFunction|TryWallSliding)
      (Variables|Default|SetCounterCooldown (- (Variables|Default|GetCounterCooldown) (Utilities|Time|GetWorldDeltaSeconds)))
      (Utilities|FlowControl|Sequence
        (:then_0
          (if (not (Variables|/Game/Blueprints/Characters/BPC_Vitality.BPC_Vitality_C|GetIsDefeated (Variables|Default|GetBPC_Vitality)))
            (Utilities|FlowControl|DoOnce false :!label _label
              (:Completed
                (Variables|Default|SetBaseLateralFriction (Variables|/Script/Engine.CharacterMovementComponent|GetFallingLateralFriction (Variables|Character|GetCharacterMovement)))
                (Variables|Default|SetBaseRunSpeed (Class|MovementComponent|GetMaxSpeed (Variables|Character|GetCharacterMovement)))
                (Variables|Default|SetDashCooldown 0.0)
                (Variables|Default|SetFaction "NewEnumerator0")
                (Variables|Default|SetBaseGravity (Variables|/Script/Engine.CharacterMovementComponent|GetGravityScale (Variables|Character|GetCharacterMovement)))))
            (elif (Variables|/Game/Blueprints/Characters/BPC_Vitality.BPC_Vitality_C|GetIsDefeated (Variables|Default|GetBPC_Vitality))
              (goto _label Reset))))
        (:then_1
          (Utilities|FlowControl|Delay 3.0)
          (Variables|/Game/Blueprints/Characters/BPC_Vitality.BPC_Vitality_C|SetCurrentStamina _bpc_vitality (Math|Float|Clamp(Float) (+ 1.0 (Variables|/Game/Blueprints/Characters/BPC_Vitality.BPC_Vitality_C|GetCurrentStamina _bpc_vitality)) 0.0 (Variables|/Game/Blueprints/Characters/BPC_Vitality.BPC_Vitality_C|GetMaxStamina _bpc_vitality))))))))

(event Game|Damage|EventAnyDamage
  (params (Damage :type Float%20%28single-precision%29) (DamageType :type Damage%20Type%20Object%20Reference) (InstigatedBy :type Controller%20Object%20Reference) (DamageCauser :type Actor%20Object%20Reference))
  (bind _bpc_vitality (Variables|Default|GetBPC_Vitality))
  (if (or (>= (- (Variables|Default|GetStaminaBlockCost) 1.0) (Variables|/Game/Blueprints/Characters/BPC_Vitality.BPC_Vitality_C|GetCurrentStamina (Variables|Default|GetBPC_Vitality))) (not (Variables|Default|GetIsBlocking)))
    (if (Variables|Default|GetIsCountering)
      (CallFunction|DeflectProjectile)
      (else
        (|CallParentFunction Damage 0 0 0)
        (Default|UpdateHealth (Variables|/Game/Widgets/WBP_HUD.WBP_HUD_C|GetWBP_HealthComponent (Variables|/Game/Blueprints/GM_Action.GM_Action_C|GetHudWidget (Variables|Default|GetGM%20Action))) (Variables|/Game/Blueprints/Characters/BPC_Vitality.BPC_Vitality_C|GetCurrentHealth (Variables|Default|GetBPC_Vitality)))
        (|RespawnSequence)))
    (else
      (Variables|/Game/Blueprints/Characters/BPC_Vitality.BPC_Vitality_C|SetCurrentStamina _bpc_vitality (- (Variables|/Game/Blueprints/Characters/BPC_Vitality.BPC_Vitality_C|GetCurrentStamina _bpc_vitality) (Variables|Default|GetStaminaBlockCost))))))

(fn ConstructionScript
  (|CallParentFunction))

(fn TryWallSliding
  (bind _returnvalue (Transformation|GetActorLocation))
  (if (and (|IsDescending_2) (|IsHoldingTowardsWall_2))
    (bind _returnvalue_2 (Collision|LineTraceForObjects _returnvalue (+ _returnvalue (* (Transformation|GetActorForwardVector) (Variables|Default|GetWallTraceLength))) (Utilities|Array|MakeArray "ObjectTypeQuery1") false 0 "None"))
    (if _returnvalue_2
      (Variables|Default|SetIsWallSliding true)
      (Variables|/Script/Engine.MovementComponent|SetVelocity (Variables|Character|GetCharacterMovement) (Math|Vector|MakeVector (.x (Variables|/Script/Engine.MovementComponent|GetVelocity (Variables|Character|GetCharacterMovement))) (.y (Variables|/Script/Engine.MovementComponent|GetVelocity (Variables|Character|GetCharacterMovement))) (Math|Float|Max(Float) (.z (Variables|/Script/Engine.MovementComponent|GetVelocity (Variables|Character|GetCharacterMovement))) (Variables|Default|GetWallSlideSpeed))))
      (else
        (Variables|Default|SetIsWallSliding false)))
    (else
      (Variables|Default|SetIsWallSliding false))))

(fn AfterRes\
  (Variables|Default|SetBaseLateralFriction (Variables|/Script/Engine.CharacterMovementComponent|GetFallingLateralFriction (Variables|Character|GetCharacterMovement)))
  (Variables|Default|SetBaseRunSpeed (Class|MovementComponent|GetMaxSpeed (Variables|Character|GetCharacterMovement)))
  (Variables|Default|SetDashCooldown 0.0)
  (Variables|Default|SetFaction "NewEnumerator0")
  (Variables|Default|SetBaseGravity (Variables|/Script/Engine.CharacterMovementComponent|GetGravityScale (Variables|Character|GetCharacterMovement))))

(fn DeflectProjectile
  (bind _counter (Variables|Default|GetCounter))
  (Game|SpawnActorfromClass "/Game/Blueprints/Projectiles/BP_ProjectilePlayer.BP_ProjectilePlayer_C" (Math|Transform|MakeTransform (Transformation|GetWorldLocation _counter) (Transformation|GetWorldRotation _counter) "1.000000,1.000000,1.000000") "AlwaysSpawn" "MultiplyWithRoot" 0 0))