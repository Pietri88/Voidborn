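; Base 2D character Blueprint that handles damage, death, hit flash and attack and jump cooldown timers.
; Tick counts both cooldowns down and derives the jump cooldown flag.
; Damage goes to BPCVitality until defeated; zero health jumps the animation instance to death and makes the capsule ignore pawns.
; Surviving hits tint the sprite through a dynamic material, with a timeline fading the flash multiplier to zero.
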(event Custom|TriggerFlash
  (params (FlashColor :type Linear%20Color%20Structure) (FlashMultiplier :type Float%20%28single-precision%29))
  (Rendering|Material|SetScalarParameterValue (Variables|Default|GetDynamicSpriteMat) "FlashMultiplier" FlashMultiplier :!class /Script/Engine.MaterialInstanceDynamic)
  (Rendering|Material|SetVectorParameterValue (Variables|Default|GetDynamicSpriteMat) "FlashColor" FlashColor :!class /Script/Engine.MaterialInstanceDynamic)
  (Components|Timeline|SetPlayRate (Variables|Default|GetSprite) (Variables|Default|GetSpriteFlashPlayRate))
  (bind _alpha (Timeline|FadeSpriteFlash PlayFromStart)
    (:Update
      (Rendering|Material|SetScalarParameterValue (Variables|Default|GetDynamicSpriteMat) "FlashMultiplier" (Math|Float|Lerp FlashMultiplier 0.0 _alpha) :!class /Script/Engine.MaterialInstanceDynamic))))

(event EventBeginPlay
  (bind _returnvalue (Rendering|Material|CreateDynamicMaterialInstance (Variables|Default|GetSprite) 0 0 "None" :!class /Script/Engine.PrimitiveComponent))
  (Variables|Default|SetDynamicSpriteMat _returnvalue)
  (Variables|Default|SetAttackCooldown 0.0))

(event Collision|EventActorBeginOverlap
  (params (OtherActor :type Actor%20Object%20Reference)))

(event EventTick
  (params (DeltaSeconds :type Float%20%28single-precision%29))
  (Variables|Default|SetAttackCooldown (- (Variables|Default|GetAttackCooldown) (Utilities|Time|GetWorldDeltaSeconds)))
  (Variables|Default|SetJumpCooldown (- (Variables|Default|GetJumpCooldown) (Utilities|Time|GetWorldDeltaSeconds)))
  (if (<= (Variables|Default|GetJumpCooldown) 0.0)
    (Variables|Default|SetJumpOnCooldown false)
    (else
      (Variables|Default|SetJumpOnCooldown true))))

(event Game|Damage|EventAnyDamage
  (params (Damage :type Float%20%28single-precision%29) (DamageType :type Damage%20Type%20Object%20Reference) (InstigatedBy :type Controller%20Object%20Reference) (DamageCauser :type Actor%20Object%20Reference))
  (if (not (Variables|/Game/Blueprints/Characters/BPC_Vitality.BPC_Vitality_C|GetIsDefeated (Variables|Default|GetBPC_Vitality)))
    (Default|ReceiveDamage (Variables|Default|GetBPC_Vitality) Damage)
    (if (<= (Variables|/Game/Blueprints/Characters/BPC_Vitality.BPC_Vitality_C|GetCurrentHealth (Variables|Default|GetBPC_Vitality)) 0.0)
      (Variables|Default|SetIsDead true)
      (Class|PaperZDAnimInstance|JumptoNode (Variables|/Script/PaperZD.PaperZDAnimationComponent|GetAnimInstance (Variables|Default|GetAnimationComponent)) "JumpDeath" "None")
      (Collision|SetCollisionResponsetoChannel (Variables|Default|GetCapsuleComponent) "ECC_Pawn" "ECR_Ignore")
      (else
        (CallFunction|TriggerFlash "(R=1.000000,G=0.061979,B=0.091826,A=1.000000)" 1e+01)))))

(fn ConstructionScript)