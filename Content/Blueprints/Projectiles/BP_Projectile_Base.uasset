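; Base projectile actor that damages characters of an opposing faction.
; A sphere overlap casts the other actor to the base character, compares factions, then applies the projectile's damage and destroys itself when they differ.
; Overlaps with same-faction characters or non-character actors are ignored, while any blocking hit on the sphere destroys the projectile without dealing damage.
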(event OnComponentHit(Sphere)
  (params (HitComponent :type Primitive%20Component%20Object%20Reference) (OtherActor :type Actor%20Object%20Reference) (OtherComp :type Primitive%20Component%20Object%20Reference) (NormalImpulse :type Vector :default "0, 0, 0") (Hit :type Hit%20Result%20Structure%20%28by%20ref%29))
  (Actor|DestroyActor))

(event OnComponentBeginOverlap(Sphere)
  (params (OverlappedComponent :type Primitive%20Component%20Object%20Reference) (OtherActor :type Actor%20Object%20Reference) (OtherComp :type Primitive%20Component%20Object%20Reference) (OtherBodyIndex :type Integer) (bFromSweep :type Boolean) (SweepResult :type Hit%20Result%20Structure%20%28by%20ref%29))
  (bind _asbp_base_character (Utilities|Casting|CastToBP_BASE_CHARACTER OtherActor))
  (if (Utilities|Enum|NotEqual(Enum) (Variables|/Game/Blueprints/Characters/BP_BASE_CHARACTER.BP_BASE_CHARACTER_C|GetFaction _asbp_base_character) (Variables|Default|GetFaction))
    (Game|Damage|ApplyDamage _asbp_base_character (Variables|Default|GetProjectileDamage) 0 self)
    (Actor|DestroyActor)))

(event EventBeginPlay)

(event Collision|EventActorBeginOverlap
  (params (OtherActor :type Actor%20Object%20Reference)))

(event EventTick
  (params (DeltaSeconds :type Float%20%28single-precision%29)))

(fn ConstructionScript)