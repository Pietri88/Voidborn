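; BP_Checkpoint is a checkpoint prop that becomes the game's active checkpoint when BP_Player first enters its Trigger.
; A DoOnce limits activation to one time, registering the actor on the GM_Action game mode cached at BeginPlay.
; Activation logs a GameAnalytics progression event with checkpoint name, death count and game time as score.
; It then tints the Paper sprite green and plays a 2D sound.
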(event OnComponentBeginOverlap(Trigger)
  (params (OverlappedComponent :type Primitive%20Component%20Object%20Reference) (OtherActor :type Actor%20Object%20Reference) (OtherComp :type Primitive%20Component%20Object%20Reference) (OtherBodyIndex :type Integer) (bFromSweep :type Boolean) (SweepResult :type Hit%20Result%20Structure%20%28by%20ref%29))
  (bind _gmaction (Variables|Default|GetGmAction))
  (Utilities|Casting|CastToBP_Player OtherActor)
  (Utilities|FlowControl|DoOnce false
    (:Completed
      (bind _output_get (Variables|/Game/Blueprints/GM_Action.GM_Action_C|SetActiveCheckpoint _gmaction self))
      (Class|GameAnalytics|AddProgressionEventwithScore (Variables|/Game/Blueprints/GM_Action.GM_Action_C|GetGameAnalytics _gmaction) "complete" (Math|Float|Truncate (Utilities|Time|GetGameTimeinSeconds)) (Utilities|GetDisplayName _output_get) (Utilities|String|Append "Deaths: " (Utilities|String|ToString(Integer) (Variables|/Game/Blueprints/GM_Action.GM_Action_C|GetDeathsCount (Variables|Default|GetGmAction)))) "" "(Values=)" false)
      (if true
        (Sprite|SetSpriteColor (Variables|Default|GetPaperSprite) "(R=0.372549,G=1.000000,B=0.341176,A=1.000000)")
        (Audio|PlaySound2D "/Game/Sounds/Fantasy_UI_SFX/Fantasy_UI_SFX/Fantasy/Fantasy_UI__18_.Fantasy_UI__18_" 1.0 1.0 0.0 0 0)))))

(event EventBeginPlay
  (bind _asgm_action (Utilities|Casting|CastToGM_Action (Game|GetGameMode)))
  (Variables|Default|SetGmAction _asgm_action))

(event Collision|EventActorBeginOverlap
  (params (OtherActor :type Actor%20Object%20Reference)))

(event EventTick
  (params (DeltaSeconds :type Float%20%28single-precision%29)))

(fn ConstructionScript)