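; BP_BossZone is a trigger zone that shows the boss health bar while the player is inside it.
; Every tick it looks up a BP_Boss actor in the level with GetActorOfClass and caches it as BossRef.
; When player 0's BP_Player begins overlapping, it tells that player to spawn a health bar for BossRef, and removes the bar when the overlap ends.
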(event EventBeginPlay)

(event Collision|EventActorBeginOverlap
  (params (OtherActor :type Actor%20Object%20Reference))
  (bind _asbp_player (Utilities|Casting|CastToBP_Player (Game|GetPlayerCharacter 0)))
  (if (== _asbp_player OtherActor)
    (Default|SpawnBossHealthBar _asbp_player (Variables|Default|GetBossRef))))

(event EventTick
  (params (DeltaSeconds :type Float%20%28single-precision%29))
  (bind _returnvalue (Actor|GetActorOfClass "/Game/Blueprints/Characters/Enemy/Boss/BP_Boss.BP_Boss_C"))
  (Variables|Default|SetBossRef _returnvalue))

(event Collision|EventActorEndOverlap
  (params (OtherActor :type Actor%20Object%20Reference))
  (bind _asbp_player (Utilities|Casting|CastToBP_Player (Game|GetPlayerCharacter 0)))
  (if (== _asbp_player OtherActor)
    (Default|RemoveBossHealthBar _asbp_player)))

(fn ConstructionScript)